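; Coin-operated switch that opens a linked BP_Door when the player interacts with it.
; Its box overlap registers it as the character's Interactable and toggles a text label showing the coin cost.
; Interact deducts CoinToUse and opens the door if the player has any coins (not necessarily enough), otherwise a timeline tints the text between white and red.
; Once opened, further interaction only displays a French "door is open" message.
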(event `self.ReceiveBeginPlay`
  (bind _textrender (`self.TextRender`))
  ; Set Text
  (`TextRenderComponent.K2_SetText` _textrender (`KismetTextLibrary.Conv_StringToText` (`KismetStringLibrary.Concat_StrStr` (`KismetTextLibrary.Conv_TextToString` (`TextRenderComponent.Text` _textrender)) (`KismetStringLibrary.Conv_IntToString` (`KismetMathLibrary.Round` (`self.coinToUse`))) " pièces"))))

(event `self.Interact`
  (if (`self.doorOpened`)
    (`TextRenderComponent.K2_SetText` (`self.TextRender`) (`KismetTextLibrary.Conv_StringToText` "La porte est ouverte"))
    (else
      (bind _asbp_third_person_character (cast `/Game/Trash/ThirdPerson/Blueprints/BP_ThirdPersonCharacter` (`GameplayStatics.GetPlayerCharacter` 0)))
      (if (> (`/Game/Trash/ThirdPerson/Blueprints/BP_ThirdPersonCharacter.CoinCounter` _asbp_third_person_character) 0.0)
        (`/Game/Trash/ThirdPerson/Blueprints/BP_ThirdPersonCharacter.AddCoin` _asbp_third_person_character (* (`self.coinToUse`) -1.0))
        (bind _asbp_door (cast `/Game/Trash/BP_Door` (`self.doorToOpen`)))
        (`/Game/Trash/BP_Door.Open` _asbp_door)
        (set `self.doorOpened` true)
        (else
          (bind (_direction _gb) (`Timeline|Timeline` :!via `PlayFromStart`)
            (:`Update`
              (bind _returnvalue (`KismetMathLibrary.Lerp` 1.0 0.0 _gb))
              (`TextRenderComponent.SetTextRenderColor` (`self.TextRender`) (`KismetMathLibrary.Conv_LinearColorToColor` (`KismetMathLibrary.MakeColor` 1.0 _returnvalue _returnvalue))))))))))

(event `self.Box.OnComponentBeginOverlap`
  (params (OverlappedComponent :type "PrimitiveComponent Object Reference") (OtherActor :type "Actor Object Reference") (OtherComp :type "PrimitiveComponent Object Reference") (OtherBodyIndex :type Integer) (bFromSweep :type Boolean) (SweepResult :type "HitResult Structure (by ref)"))
  (bind _asbp_third_person_character (cast `/Game/Trash/ThirdPerson/Blueprints/BP_ThirdPersonCharacter` OtherActor))
  (set `/Game/Trash/ThirdPerson/Blueprints/BP_ThirdPersonCharacter.Interactable` self _asbp_third_person_character)
  (`SceneComponent.SetVisibility` (`self.TextRender`) true false))

(event `self.Box.OnComponentEndOverlap`
  (params (OverlappedComponent :type "PrimitiveComponent Object Reference") (OtherActor :type "Actor Object Reference") (OtherComp :type "PrimitiveComponent Object Reference") (OtherBodyIndex :type Integer))
  (bind _asbp_third_person_character (cast `/Game/Trash/ThirdPerson/Blueprints/BP_ThirdPersonCharacter` OtherActor))
  (set `/Game/Trash/ThirdPerson/Blueprints/BP_ThirdPersonCharacter.Interactable` null _asbp_third_person_character)
  (`SceneComponent.SetVisibility` (`self.TextRender`) false false))

(fn `UserConstructionScript`
  (`parent.UserConstructionScript`))