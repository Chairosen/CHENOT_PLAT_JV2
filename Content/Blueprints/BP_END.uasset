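; BP_END is a level-end trigger that sends the player to the L_EndScreen level when they enter its box.
; On overlap by BP_ThirdPersonCharacter, it waits briefly, drops its cube downward and destroys the trigger box so it fires once.
; The EndGame event then clears all widgets and opens the end screen level after a short delay.
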(event `EndGame`
  (`WidgetLayoutLibrary.RemoveAllWidgets`)
  (`KismetSystemLibrary.Delay` 0.5)
  (`GameplayStatics.OpenLevelBySoftObjectPtr` "/Game/Level/L_EndScreen.L_EndScreen"))

(event `self.Box.OnComponentBeginOverlap`
  (params (OverlappedComponent :type "PrimitiveComponent Object Reference") (OtherActor :type "Actor Object Reference") (OtherComp :type "PrimitiveComponent Object Reference") (OtherBodyIndex :type Integer) (bFromSweep :type Boolean) (SweepResult :type "HitResult Structure (by ref)"))
  (cast `/Game/Trash/ThirdPerson/Blueprints/BP_ThirdPersonCharacter` OtherActor)
  (`KismetSystemLibrary.Delay` 0.2)
  (`SceneComponent.K2_AddLocalOffset` (`self.Cube`) (0.0 0.0 -200.0) false false)
  (`ActorComponent.K2_DestroyComponent` (`self.Box`))
  (`self.EndGame`))

(fn `UserConstructionScript`
  (`parent.UserConstructionScript`))